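; Lockable child door Blueprint that blocks opening while locked and shows its state through a red or green indicator light.
; Interact toggles an unlocked door, or checks the overlapping actor's BP_BackpackComponent for the required key items when locked.
; Matching keys are removed as found, even if the set is incomplete, and the door unlocks only when all match.
; Lock only takes effect on doors without required keys, while SwitchLock and Unlock ignore keys.
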(event EventBeginPlay
  (|CallParentFunction) ; This node is disabled and will not be called.\nDrag off pins to build functionality.
)

(event Collision|EventActorBeginOverlap
  (params (OtherActor :type Actor%20Object%20Reference))
  (|CallParentFunction OtherActor) ; This node is disabled and will not be called.\nDrag off pins to build functionality.
)

(event EventTick
  (params (DeltaSeconds :type Float%20%28single-precision%29))
  (|CallParentFunction DeltaSeconds) ; This node is disabled and will not be called.\nDrag off pins to build functionality.
)

(event EventOpenDoor
  (if (not (Variables|DoorConfig|GetIsDoorLocked))
    (|CallParentFunction)))

(event EventCloseDoor
  (|CallParentFunction))

(fn ConstructionScript
  (|CallParentFunction)
  (CallFunction|UpdateDoorLockIndecation))

(fn SwitchLock
  (Variables|DoorConfig|SetIsDoorLocked (not (Variables|DoorConfig|GetIsDoorLocked)))
  (CallFunction|UpdateDoorLockIndecation))

(fn UpdateDoorLockIndecation
  (Rendering|Components|Light|SetLightColor (Variables|Default|GetLockIndicatorLight) (Math|Color|SelectColor "(R=1.000000,G=0.041667,B=0.041667,A=1.000000)" "(R=0.000000,G=1.000000,B=0.089136,A=1.000000)" (Variables|DoorConfig|GetIsDoorLocked)) true))

(fn Lock
  (if (not (Utilities|Array|IsValidIndex (Variables|Default|GetNeededKeysName)))
    (Variables|DoorConfig|SetIsDoorLocked true)
    (CallFunction|UpdateDoorLockIndecation)))

(fn Unlock
  (Variables|DoorConfig|SetIsDoorLocked false)
  (CallFunction|UpdateDoorLockIndecation))

(fn Interact
  (if (Variables|Default|GetIsReadyToInteract)
    (if (not (Variables|DoorConfig|GetIsDoorLocked))
      (if (Variables|Default|GetIsDoorOpen)
        (CallFunction|CloseDoor)
        (return true)
        (else
          (CallFunction|OpenDoor)
          (return true)))
      (elif (Utilities|Array|IsValidIndex (Variables|Default|GetNeededKeysName))
        (bind _overlappedactor (Variables|Default|GetOverlappedActor)
          (:then
            (Utilities|IsValid (Actor|GetComponentbyClass _overlappedactor "/Game/BP/Components/BP_BackpackComponent.BP_BackpackComponent_C")
              (:Is%20Valid
                (LocalVariables|SetL_Backpack (Actor|GetComponentbyClass _overlappedactor "/Game/BP/Components/BP_BackpackComponent.BP_BackpackComponent_C"))
                (for _array_element (Variables|Default|GetNeededKeysName)
                  (LocalVariables|SetL_ItemName _array_element)
                  (if (Utilities|Set|Contains (Variables|/Game/BP/Components/BP_BackpackComponent.BP_BackpackComponent_C|GetQuestItems (LocalVariables|GetL_Backpack)) (LocalVariables|GetL_ItemName))
                    (Math|Integer|IncrementInt (LocalVariables|GetL_ItemIntement)
                      (:%20%20
                        ;[0.1002 0.6952 1] If you can to remove item from inventory after use
                        (Utilities|Set|Remove (Variables|/Game/BP/Components/BP_BackpackComponent.BP_BackpackComponent_C|GetQuestItems (LocalVariables|GetL_Backpack)) (LocalVariables|GetL_ItemName))))))
                (if (== (LocalVariables|GetL_ItemIntement) (Utilities|Array|Length (Variables|Default|GetNeededKeysName)))
                  (CallFunction|Unlock)
                  (else
                    (return true))))
              (:Is%20Not%20Valid
                (return true))))
          (:else
            (return true)))
        (else
          (return true))))
    (else
      (return false))))