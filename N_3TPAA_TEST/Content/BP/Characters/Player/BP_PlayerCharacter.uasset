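; Player character Blueprint that extends its parent's main action so that using it emits a noise event for AI hearing.
; The ActionMain override runs the parent logic, then checks ActionMainPressed and reports a "Noise"-tagged event at the capsule's location, with itself as instigator.
; A DoOnce limits this to one report per press and resets when the flag is false.
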(event EventBeginPlay
  (|CallParentFunction))

(event Collision|EventActorBeginOverlap
  (params (OtherActor :type Actor%20Object%20Reference))
  (|CallParentFunction OtherActor) ; This node is disabled and will not be called.\nDrag off pins to build functionality.
)

(event EventTick
  (params (DeltaSeconds :type Float%20%28single-precision%29))
  (|CallParentFunction DeltaSeconds) ; This node is disabled and will not be called.\nDrag off pins to build functionality.
)

(fn ConstructionScript
  (|CallParentFunction))

(fn ActionMain
  (params (IsPressed :type Boolean))
  (|CallParentFunction IsPressed)
  (if (Variables|Default|GetActionMainPressed)
    (Utilities|FlowControl|DoOnce false :!label _label
      (:Completed
        (Class|AISenseHearing|ReportNoiseEvent (Transformation|GetWorldLocation (Variables|Default|GetCapsuleComponent)) 1.0 self 0.0 "Noise")))
    (else
      (goto _label Reset))))