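; BP_NPCCharacter is an NPC character Blueprint that displays its AI state on a tooltip text facing the player's camera.
; Each Tick flags whether the player pawn is within a set range, then LookingAtPlayerCamera writes the BP_AIController's AIStats enum to TooltipText and rotates it toward the camera.
; Outside that range the tooltip stops updating but is not hidden.
; The ActionMain override calls its parent, then prints a placeholder "Bang" message when pressed.
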(event EventBeginPlay
  (|CallParentFunction) ; This node is disabled and will not be called.\nDrag off pins to build functionality.
)

(event Collision|EventActorBeginOverlap
  (params (OtherActor :type Actor%20Object%20Reference))
  (|CallParentFunction OtherActor) ; This node is disabled and will not be called.\nDrag off pins to build functionality.
)

(event EventTick
  (params (DeltaSeconds :type Float%20%28single-precision%29))
  (|CallParentFunction DeltaSeconds)
  (Variables|Default|SetLookAtPlayerCamera (<= (Math|Vector|VectorLength (- (Transformation|GetWorldLocation (Variables|Default|GetCapsuleComponent)) (Transformation|GetActorLocation (Game|Player|GetPlayerPawn 0)))) 1.5e+03))
  (CallFunction|LookingatPlayerCamera))

(fn ConstructionScript
  (|CallParentFunction))

(fn ActionMain
  (params (IsPressed :type Boolean))
  (|CallParentFunction IsPressed)
  (if (Variables|Default|GetActionMainPressed)
    (Development|PrintString "Bang" true false "(R=1.000000,G=0.070155,B=0.030354,A=1.000000)" 1.0)))

(fn LookingatPlayerCamera
  (if (Variables|Default|GetLookAtPlayerCamera)
    (bind _asbp_aicontroller (Utilities|Casting|CastToBP_AIController (Pawn|GetController)))
    (bind _asbp_player_character (Utilities|Casting|CastToBP_PlayerCharacter (Game|Player|GetPlayerPawn 0)))
    (LocalVariables|SetCameraLocation (Transformation|GetWorldLocation (Variables|/Game/BP/Characters/Player/BP_PlayerCharacter.BP_PlayerCharacter_C|GetCamera _asbp_player_character)))
    (Rendering|Components|TextRender|SetText (Variables|Default|GetTooltipText) (Utilities|Text|FormatText "{AIState}" (Utilities|String|EnumtoString (Variables|/Game/BP/Controllers/BP_AIController.BP_AIController_C|GetAIStats _asbp_aicontroller))))
    (Transformation|SetWorldRotation (Variables|Default|GetTooltipText) (Math|Rotator|FindLookatRotation (Transformation|GetWorldLocation (Variables|Default|GetTooltipText)) (LocalVariables|GetCameraLocation)) false false)))