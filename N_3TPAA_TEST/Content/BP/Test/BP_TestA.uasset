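; Test actor Blueprint that exercises basic scripting features: custom events, functions, arrays, branches and text formatting.
; On BeginPlay it calls a custom event that prints its parameters in green or red by the bool, directly and through NewFunction0, which uses MultByFive.
; The construction script shows MyName on a TextRender component.
; A traffic-light enum sequence, a condition check and several logic nodes are left unconnected.
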(event Custom|CustomEvent_0
  (params (InNewParam :type Boolean) (InNewParam2 :type Byte) (InNewParam3 :type Float%20%28single-precision%29) (InNewParam4 :type Name))
  (Development|PrintString (Utilities|String|Append "Bool =" (Utilities|String|ToString(Boolean) InNewParam) "Float =" (Utilities|String|ToString(Float) InNewParam3) " !") true false (Math|Color|SelectColor "(R=0.000000,G=1.000000,B=0.161131,A=1.000000)" "(R=1.000000,G=0.000000,B=0.009181,A=1.000000)" InNewParam) 5.0))

(event Custom|CustomEvent_1)

(event EventBeginPlay
  (CallFunction|CustomEvent0 false 0 0.0 "None")
  (CallFunction|CustomEvent0 true 0 0.0 "None")
  (Test|NewFunction0 "None" (Utilities|Array|MakeArray true) 1))

(event Collision|EventActorBeginOverlap
  (params (OtherActor :type Actor%20Object%20Reference)))

(event EventTick
  (params (DeltaSeconds :type Float%20%28single-precision%29)))

(fn ConstructionScript
  (Rendering|Components|TextRender|SetText (Variables|Default|GetTextRender) (Utilities|Text|FormatText "my name is {Name}" (Variables|Test|GetMyName))))

(fn NewFunction0
  (params (InName :type Name) (InArray :type Array%20of%20Booleans) (InInt :type Integer))
  (bind (_result _success) (Test|MultbyFive InInt))
  (Utilities|FlowControl|Sequence
    (:then_0)
    (:then_1)
    (:then_2)
    (:then_3
      (if (Utilities|Array|Get(acopy) InArray)
        (if _success
          (LocalVariables|SetL_Int _result)
          (CallFunction|CustomEvent0 (Utilities|Array|Get(acopy) InArray) 0 (Math|Conversions|ToFloat(Integer) (LocalVariables|GetL_Int)) InName)
          (CallFunction|CustomEvent1)
          (return (LocalVariables|GetL_Int)))
        (else
          (return 0))))))

(fn NewFunction1)

(fn MultbyFive
  (params (InParam :type Integer))
  (return (* InParam 5) true))