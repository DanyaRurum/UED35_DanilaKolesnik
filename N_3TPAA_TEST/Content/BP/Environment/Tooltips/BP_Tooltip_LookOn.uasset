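; Tooltip actor whose text turns to face the player's camera while the player is in its overlap area.
; Begin overlap enables facing if PlayerInbox is valid, and any end overlap disables it.
; Each Tick, while enabled, it casts PlayerInbox to BP_PlayerCharacter and rotates TooltipText with a look-at rotation toward that character's camera.
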(event EventBeginPlay
  (|CallParentFunction) ; This node is disabled and will not be called.\nDrag off pins to build functionality.
)

(event Collision|EventActorBeginOverlap
  (params (OtherActor :type Actor%20Object%20Reference))
  (|CallParentFunction OtherActor) ; This node is disabled and will not be called.\nDrag off pins to build functionality.
)

(event EventTick
  (params (DeltaSeconds :type Float%20%28single-precision%29))
  (|CallParentFunction DeltaSeconds)
  (CallFunction|LookingatPlayerCamera))

(event EventActorBeginOverlap
  (params (OtherActor :type Actor%20Object%20Reference))
  (|CallParentFunction OtherActor)
  (Variables|Default|GetPlayerInbox
    (:then
      (Variables|Default|SetLookAtPlayerCamera true))
    (:else)))

(event EventActorEndOverlap
  (params (OtherActor :type Actor%20Object%20Reference))
  (|CallParentFunction OtherActor)
  (Variables|Default|SetLookAtPlayerCamera false))

(fn ConstructionScript
  (|CallParentFunction))

(fn LookingatPlayerCamera
  (if (Variables|Default|GetLookAtPlayerCamera)
    (bind _playerinbox (Variables|Default|GetPlayerInbox)
      (:then
        (bind _asbp_player_character (Utilities|Casting|CastToBP_PlayerCharacter _playerinbox))
        (Variables|Default|SetCameraLocation (Transformation|GetWorldLocation (Variables|/Game/BP/Characters/Player/BP_PlayerCharacter.BP_PlayerCharacter_C|GetCamera _asbp_player_character)))
        (Transformation|SetWorldRotation (Variables|Default|GetTooltipText) (Math|Rotator|FindLookatRotation (Transformation|GetWorldLocation (Variables|Default|GetTooltipText)) (Variables|Default|GetCameraLocation)) false false))
      (:else))))