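; BP_ShootingTargets is a damageable target that shows its HP on a text render and is destroyed shortly after death.
; Any character overlapping it makes it apply fixed BP_DamageObject damage to itself, crediting that character.
; Incoming damage of that type class is forwarded to BPMainStatesComponent, whose stats-updated event refreshes the text.
; On death the text announces it, then the actor destroys itself after a short delay.
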(event Custom|OnDeath
  (Utilities|FlowControl|Delay 1.0)
  (Actor|DestroyActor))

(event EventBeginPlay
  (bind _bp_mainstatescomponent (Variables|Default|GetBP_MainStatesComponent))
  (EventDispatchers|BindEventtoOnStatsUpdated (Variables|Default|GetBP_MainStatesComponent) (EventDispatchers|CreateEvent :!event OnStatsUpdated))
  (CallFunction|OnStatsUpdated (Variables|/Game/BP/Components/BP_MainStatesComponent.BP_MainStatesComponent_C|GetCurrentHP _bp_mainstatescomponent) (Variables|/Game/BP/Components/BP_MainStatesComponent.BP_MainStatesComponent_C|GetCurrentEP _bp_mainstatescomponent) false false))

(event Collision|EventActorBeginOverlap
  (params (OtherActor :type Actor%20Object%20Reference))
  (bind _asbp_character_base (Utilities|Casting|CastToBP_CharacterBase OtherActor))
  (Game|Damage|ApplyDamage self 7.0 0 _asbp_character_base "/Game/BP/Objects/BP_DamageObject.BP_DamageObject_C"))

(event EventTick
  (params (DeltaSeconds :type Float%20%28single-precision%29)))

(fn ConstructionScript)

(fn ReceiveAnyDamage
  (params (Damage :type Float%20%28single-precision%29) (DamageType :type Damage%20Type%20Object%20Reference) (InstigatedBy :type Controller%20Object%20Reference) (DamageCauser :type Actor%20Object%20Reference))
  (bind _asbp_damage_object (Utilities|Casting|CastToBP_DamageObject DamageType))
  (Default|ReceiveDamage (Variables|Default|GetBP_MainStatesComponent) Damage (Variables|/Game/BP/Objects/BP_DamageObject.BP_DamageObject_C|GetDamageType _asbp_damage_object) DamageCauser))

(fn OnStatsUpdated
  (params (CurrentHP :type Integer) (CurrentEP :type Integer) (IsDead :type Boolean) (isItDamage :type Boolean))
  (bind _bp_mainstatescomponent (Variables|Default|GetBP_MainStatesComponent))
  (Rendering|Components|TextRender|SetText (Variables|Default|GetTextRender) (select IsDead (Utilities|Text|FormatText "{a} Is Dead" (Utilities|GetDisplayName self)) (Utilities|Text|FormatText "HP {hp}/{Maxhp}" (Variables|/Game/BP/Components/BP_MainStatesComponent.BP_MainStatesComponent_C|GetCurrentHP _bp_mainstatescomponent) (Utilities|Struct|BreakSTRUCT_MainStats (Variables|/Game/BP/Components/BP_MainStatesComponent.BP_MainStatesComponent_C|GetMainStatsStructure _bp_mainstatescomponent)))))
  (if IsDead
    (CallFunction|OnDeath)))